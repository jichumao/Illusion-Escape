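; Game state for a humans-versus-AI hacking match that tracks hack progress and triggers each side's win screen.
; Two or more hacks trigger the human win, while Twister hack progress climbing in steps to full triggers the AI win.
; Multicast events create the win widgets with a mouse cursor and show or hide a reusable client hacking widget.
; Hack count changes also toggle the swap skill on player controller 0.
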(event Custom|Multicast_ShowHumanWinUI
  (bind _returnvalue (UserInterface|CreateWidget "/Game/UI/UI_HumanWin.UI_HumanWin_C"))
  (UserInterface|Viewport|AddtoViewport _returnvalue 0)
  (Variables|/Script/Engine.PlayerController|SetbShowMouseCursor (Game|GetPlayerController 0) true))

(event Custom|Multicast_showHackProgress
  (Utilities|IsValid (Variables|Default|GetUI_ClicentHacking)
    (:Is%20Valid
      (Widget|SetVisibility (Variables|Default|GetUI_ClicentHacking) "Visible"))
    (:Is%20Not%20Valid
      (bind _returnvalue (UserInterface|CreateWidget "/Game/UI/UI_ClientHacking.UI_ClientHacking_C"))
      (bind _output_get (Variables|Default|SetUI_ClicentHacking _returnvalue))
      (UserInterface|Viewport|AddtoViewport _output_get 0))))

(event Custom|Multicast_hideHackProgress
  (Widget|SetVisibility (Variables|Default|GetUI_ClicentHacking) "Hidden"))

(event Custom|Multicast_ShowAIWinUI
  (bind _returnvalue (UserInterface|CreateWidget "/Game/UI/UI_AIWin.UI_AIWin_C"))
  (UserInterface|Viewport|AddtoViewport _returnvalue 0)
  (Variables|/Script/Engine.PlayerController|SetbShowMouseCursor (Game|GetPlayerController 0) true))

(event EventBeginPlay)

(event EventTick
  (params (DeltaSeconds :type Float%20%28single-precision%29)))

(fn ConstructionScript)

(fn IncreaseHackedNum
  (bind _result (Math|Integer|IncrementInt (Variables|Default|GetHackedNum))
    (:%20%20
      (CallFunction|TurnonSwapSkill)
      (bind _output_get (Variables|Default|SetHackedNum _result))
      (Development|PrintText (Utilities|Text|ToText(Integer) _output_get))
      (if (>= _output_get 2)
        (CallFunction|MulticastShowHumanWinUI)))))

(fn DecreaseHackedNum
  (bind _result (Math|Integer|DecrementInt (Variables|Default|GetHackedNum))
    (:%20%20
      (if (== (Variables|Default|GetHackedNum) 0)
        (CallFunction|TurnOffSwapSkill)
        (Variables|Default|SetHackedNum _result)))))

(fn IncreaseTwisterHackedProgress
  (bind _output_get (Variables|Default|SetTwisterHackedProgress (+ (Variables|Default|GetTwisterHackedProgress) 0.1)))
  (if (>= _output_get 1.0)
    (CallFunction|MulticastShowAIWinUI)))

(fn DecreseTwisterHackedProgress
  (bind _output_get (Variables|Default|SetTwisterHackedProgress (- (Variables|Default|GetTwisterHackedProgress) 0.1)))
  (if (<= _output_get 0.0)
    _))

(fn TurnonSwapSkill
  (bind _asbp_new_player_controller (Utilities|Casting|CastToBP_NewPlayerController (Game|GetPlayerController 0)))
  (Variables|/Game/Blueprints/BP_NewPlayerController.BP_NewPlayerController_C|SetClient_canSwapSkill _asbp_new_player_controller true)
  (Default|ChangeSwapSkill _asbp_new_player_controller)
  (Development|PrintText "Change    in game stateHello"))

(fn TurnOffSwapSkill
  (bind _asbp_new_player_controller (Utilities|Casting|CastToBP_NewPlayerController (Game|GetPlayerController 0)))
  (Variables|/Game/Blueprints/BP_NewPlayerController.BP_NewPlayerController_C|SetClient_canSwapSkill _asbp_new_player_controller false)
  (Default|ChangeSwapSkill _asbp_new_player_controller))