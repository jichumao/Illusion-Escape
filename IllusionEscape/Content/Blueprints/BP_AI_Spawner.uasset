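; BP_AI_Spawner populates the level with BP_Dummy_NPC actors when play begins.
; It gathers TargetPoints tagged RobotSpawnPoint, then spawns MaxSpawnCount NPCs, each at the location of a randomly picked point.
; Picks can repeat, so several NPCs may share a point, and only location is taken from it, not rotation.
; Two debug prints of the index range are left unconnected.
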(event EventBeginPlay
  (bind _outactors (Actor|GetAllActorsOfClasswithTag "/Script/Engine.TargetPoint" "RobotSpawnPoint"))
  (Variables|Default|SetSpawnPoints _outactors)
  (for _index (range 0 (- (Variables|Default|GetMaxSpawnCount) 1))
    (Game|SpawnActorfromClass "/Game/ThirdPerson/Blueprints/BP_Dummy_NPC.BP_Dummy_NPC_C" (Math|Conversions|ToTransform(Vector) (Transformation|GetActorLocation (Utilities|Array|Get(acopy) (Variables|Default|GetSpawnPoints) (Math|Random|RandomIntegerinRange 0 (- (Utilities|Array|Length (Variables|Default|GetSpawnPoints)) 1))))) "Undefined" "MultiplyWithRoot" 0 0)))

(fn ConstructionScript)