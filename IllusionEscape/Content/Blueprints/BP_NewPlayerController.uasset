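; Player controller that sets up the minimap and hosts three skills: position swap, screen blind and monitor break.
; On BeginPlay, local controllers add child actor components, with an extra one and IsClient set when the game mode's PlayerCounter isn't 1.
; Server-prefixed events swap BP_ClientCharacter with a random dummy NPC, break monitors on randomly picked Interaction_Boxes, or relay blind through BP_CustomGameMode.
; Event_SkillBlind displays the UI_ObservorBlind overlay.
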(event Custom|Run_On_Server)

(event Custom|Server_SkillSwap
  (CallFunction|SkillSwap))

(event Custom|Event_SkillBlind
  (CallFunction|SkillBlind))

(event Custom|Server_SkillBlind
  (bind _returnvalue (Actor|GetActorOfClass "/Game/Blueprints/BP_CustomGameMode.BP_CustomGameMode_C"))
  (Default|ClientSkillBlind _returnvalue))

(event Custom|Server_BreakMonitor
  (CallFunction|SkillBreakMonitor))

(event EventBeginPlay
  (bind _returnvalue (UserInterface|CreateWidget "/Game/UI/UI_Minimap.UI_Minimap_C"))
  (UserInterface|Viewport|AddtoViewport _returnvalue 0)
  (if (Pawn|IsLocalController)
    (AddComponent|AddChildActorComponent false)
    (bind _returnvalue_2 (Actor|GetActorOfClass "/Game/Blueprints/BP_CustomGameMode.BP_CustomGameMode_C"))
    (if (not (== (Variables|/Game/Blueprints/BP_CustomGameMode.BP_CustomGameMode_C|GetPlayerCounter _returnvalue_2) 1))
      (Development|PrintString "is client")
      (AddComponent|AddChildActorComponent false)
      (Variables|Default|SetIsClient true))))

(event EventTick
  (params (DeltaSeconds :type Float%20%28single-precision%29)))

(fn ConstructionScript)

(fn SkillSwap
  (bind _returnvalue (Actor|GetActorOfClass "/Game/ThirdPerson/Blueprints/BP_ClientCharacter.BP_ClientCharacter_C"))
  (LocalVariables|Setplayer _returnvalue)
  (bind _outactors (Actor|GetAllActorsOfClass "/Game/ThirdPerson/Blueprints/BP_Dummy_NPC.BP_Dummy_NPC_C"))
  (LocalVariables|SetTargetNpc (.OutItem (Utilities|Array|Random _outactors)))
  (LocalVariables|SetPlayerPosition (Transformation|GetActorLocation (LocalVariables|Getplayer)))
  (bind _output_get (LocalVariables|SetTargetNpcPosition (Transformation|GetActorLocation (LocalVariables|GetTargetNpc))))
  (Transformation|SetActorLocation (LocalVariables|Getplayer) _output_get false false)
  (Transformation|SetActorLocation (LocalVariables|GetTargetNpc) (LocalVariables|GetPlayerPosition) false false))

(fn SkillBlind
  (bind _returnvalue (UserInterface|CreateWidget "/Game/UI/Skill/UI_ObservorBlind.UI_ObservorBlind_C" (Game|GetPlayerController 0)))
  (UserInterface|Viewport|AddtoViewport _returnvalue 0))

(fn SkillBreakMonitor
  (bind _outactors (Actor|GetAllActorsOfClass "/Game/UI/Interaction/Interaction_Box.Interaction_Box_C"))
  (Default|BreakMonitor (.OutItem (Utilities|Array|Random _outactors)))
  (Variables|/Game/UI/Interaction/Interaction_Box.Interaction_Box_C|SetPrepareBreak (.OutItem (Utilities|Array|Random _outactors)) false))