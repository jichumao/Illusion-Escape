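; BP_GameState is a game state Blueprint that tracks how many hacks have been completed and triggers the win screen.
; IncreaseHackedNum increments HackedNum and, once it reaches five or more, creates a UI_Win widget and adds it to the viewport.
; DecreaseHackedNum decrements the counter, and no BeginPlay or Tick logic runs.
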(event EventBeginPlay)

(event EventTick
  (params (DeltaSeconds :type Float%20%28single-precision%29)))

(fn ConstructionScript)

(fn IncreaseHackedNum
  (bind _result (Math|Integer|IncrementInt (Variables|Default|GetHackedNum))
    (:%20%20
      (bind _output_get (Variables|Default|SetHackedNum _result))
      (if (>= _output_get 5)
        (bind _returnvalue (UserInterface|CreateWidget "/Game/UI/UI_Win.UI_Win_C"))
        (UserInterface|Viewport|AddtoViewport _returnvalue 0)))))

(fn DecreaseHackedNum
  (bind _result (Math|Integer|DecrementInt (Variables|Default|GetHackedNum))
    (:%20%20
      (Variables|Default|SetHackedNum _result))))